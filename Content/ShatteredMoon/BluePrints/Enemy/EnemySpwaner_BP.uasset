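; Enemy spawner Blueprint that places random enemy types inside a box volume, up to a population cap.
; Its SpawnEnemy event counts every EnemyPawn_BP actor in the level and proceeds only while the count is below MaxEnemies.
; It then spawns an AI pawn of a random EnemyList class at a random point within SpawnVolume's scaled bounds.
; Nothing in this Blueprint calls SpawnEnemy.
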(event `SpawnEnemy`
  (bind _spawnvolume (`self.SpawnVolume`))
  (bind _enemylist (`self.EnemyList`))
  (bind _outactors (`GameplayStatics.GetAllActorsOfClass` "/Game/ShatteredMoon/BluePrints/Enemy/EnemyPawn_BP.EnemyPawn_BP_C"))
  (if (< (`KismetArrayLibrary.Array_Length` _outactors) (`self.MaxEnemies`))
    (`AIBlueprintHelperLibrary.SpawnAIFromClass` (`|GetArrayItem` _enemylist (`KismetMathLibrary.RandomInteger` (`KismetArrayLibrary.Array_Length` _enemylist))) null (`KismetMathLibrary.RandomPointInBoundingBox` (`SceneComponent.K2_GetComponentLocation` _spawnvolume) (`BoxComponent.GetScaledBoxExtent` _spawnvolume)))))

(fn `UserConstructionScript`)
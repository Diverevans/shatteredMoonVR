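; Game mode for a VR wave-survival game that runs the tutorial, enemy waves, player health and win or death ending.
; Holding the start button clears unheld tutorial items and begins timed wolf spawning at random spawn points.
; Tick uses kill counts to trigger burst waves adding wasps and raising spawn caps, then declares victory or death and reloads the level.
; Helper functions rate-limit player damage and play first-pickup weapon voice lines.
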(event `self.ReceiveBeginPlay`
  (bind _outactors (`GameplayStatics.GetAllActorsOfClass` "/Game/VirtualRealityBP/Blueprints/MotionControllerPawn.MotionControllerPawn_C"))
  (set `self.VR Camera` (`|GetArrayItem` _outactors))
  (bind _outactors_2 (`GameplayStatics.GetAllActorsOfClass` "/Game/ShatteredMoon/BluePrints/Enemy/EnemySpawnPoint_BP.EnemySpawnPoint_BP_C"))
  (set `self.spawn points` _outactors_2)
  (`KismetSystemLibrary.Delay` 5.0)
  (`GameplayStatics.PlaySound2D` "/Game/ShatteredMoon/Audio/Voice/PlainGreeting_Hotton.PlainGreeting_Hotton" 1.0 1.0 0.0 null null))

(event `Key|Escape`
  (params (Key :type "Key Structure"))
  (:`Pressed`
    (`KismetSystemLibrary.QuitGame` null "Quit")))

(event `self.ReceiveTick`
  (params (DeltaSeconds :type "Float (single-precision)"))
  (bind _enemy_spawn_timer (`self.Enemy Spawn Timer`))
  (bind _vr_camera (`self.VR Camera`))
  (bind _spawn_points (`self.spawn points`))
  (bind _playerhealth (`self.playerHealth`))
  (bind _defaultsceneroot (`/Game/ShatteredMoon/BluePrints/Enemy/EnemySpawnPoint_BP.DefaultSceneRoot` (`|GetArrayItem` _spawn_points (`KismetMathLibrary.RandomInteger` (`KismetArrayLibrary.Array_Length` _spawn_points)))))
  (bind _returnvalue (`SceneComponent.K2_GetComponentLocation` _defaultsceneroot))
  (bind _returnvalue_2 (`SceneComponent.K2_GetComponentRotation` _defaultsceneroot))
  (if (<= _playerhealth 3)
    (if (not (`self.lowHealthWarning`))
      (`GameplayStatics.PlaySound2D` "/Game/ShatteredMoon/Audio/Voice/OldAudio/ShMoonLowHealth.ShMoonLowHealth" 1.0 1.0 0.0 null null)
      (set `self.lowHealthWarning` true)))
  (if (>= _playerhealth 0)
    (bind _output_get (set `self.playerCanBeHitTimer` (- (stale _output_get) DeltaSeconds))) ; player can be hit once per second
    (if (>= (`self.Enemies Killed`) 20)
      (if (`self.Wave 2`)
        (if (>= (`self.Enemies Killed`) 60)
          (if (`self.Wave 3`)
            (if (>= (`self.Enemies Killed`) 100)
              (if (`self.GameEnd`) :!label _label
                (`KismetSystemLibrary.Delay` 5.0)
                (`/Game/VirtualRealityBP/Blueprints/MotionControllerPawn.FadeOut` (`self.VR Camera`))
                (`KismetSystemLibrary.Delay` 3.0)
                (bind _returnvalue_3 (`GameplayStatics.GetCurrentLevelName` true))
                (`GameplayStatics.OpenLevel` (`KismetStringLibrary.Conv_StringToName` _returnvalue_3))
                (elif (`self.playerIsDead`)
                  (set `self.GameEnd` true) ; failure path
                  (if (<= (`KismetMathLibrary.RandomIntegerInRange` 0 100) 99)
                    (`GameplayStatics.PlaySound2D` "/Game/ShatteredMoon/Audio/Voice/YouDied.YouDied" 1.0 1.0 0.0 null null)
                    (else
                      (`GameplayStatics.PlaySound2D` "/Game/ShatteredMoon/Audio/Voice/JakeWhatHappened_Gardei.JakeWhatHappened_Gardei" 1.0 1.0 0.0 null null)))
                  (else
                    (set `self.GameEnd` true) ; victory path
                    (`GameplayStatics.PlaySound2D` "/Game/ShatteredMoon/Audio/Voice/YouWin.YouWin" 1.0 1.0 0.0 null null))))
              (else
                ;[1 1 1] Monster SPawning code.
                (if (and (<= _enemy_spawn_timer 0.0) (<= (`self.Enemy Count`) (`self.maxEnemyCount`))) :!label _label_2
                  (if true
                    (if (`self.Wave 2`)
                      ;[1 1 1] Start spawning bees on Wave 2...
                      (if (< (`self.WaspCounter`) 10)
                        (if (`KismetMathLibrary.RandomBool`)
                          (`AIBlueprintHelperLibrary.SpawnAIFromClass` "/Game/ShatteredMoon/BluePrints/Enemy/Wasp_BP.Wasp_BP_C" null _returnvalue _returnvalue_2)
                          (bind _output_get_2 (set `self.WaspCounter` (+ (stale _output_get_2) 1)))
                          (else
                            (`AIBlueprintHelperLibrary.SpawnAIFromClass` "/Game/ShatteredMoon/BluePrints/Enemy/Wolf_BP.Wolf_BP_C" null _returnvalue _returnvalue_2 :!label _label_3)))
                        (else
                          (goto _label_3)))
                      (else
                        (goto _label_3)))
                    (set `self.Enemy Spawn Timer` (`self.Enemies Per Second`))
                    (set `self.Enemy Count` (+ (`self.Enemy Count`) 1)))
                  (else
                    (set `self.Enemy Spawn Timer` (- _enemy_spawn_timer DeltaSeconds))))))
            (else
              ;[1 1 1] When Wave 3 starts, spawn a hoard and up the max monster count... Monsters will also have more health (see their individual bp's)
              (`self.burst spawn` "/Game/ShatteredMoon/BluePrints/Enemy/Wasp_BP.Wasp_BP_C" 4)
              (`self.burst spawn` "/Game/ShatteredMoon/BluePrints/Enemy/Wolf_BP.Wolf_BP_C" 4)
              (`GameplayStatics.PlaySound2D` "/Game/ShatteredMoon/Audio/Voice/OldAudio/ShMoonTemyava.ShMoonTemyava" 1.0 1.0 0.0 null null)
              (set `self.maxEnemyCount` 25) ; peformance hits start during this wave...
              (set `self.Wave 3` true)
              (set `self.Enemies Per Second` 0.4)))
          (else
            (goto _label_2)))
        (else
          ;[1 1 1] When Wave 2 starts, Spawn a bunch of Wasps
          (`self.burst spawn` "/Game/ShatteredMoon/BluePrints/Enemy/Wasp_BP.Wasp_BP_C" 8)
          (set `self.Wave 2` true)
          (set `self.maxEnemyCount` 20)
          (`GameplayStatics.PlaySound2D` "/Game/ShatteredMoon/Audio/Voice/OldAudio/ShMoonCENSOREDBEES.ShMoonCENSOREDBEES" 1.0 1.0 0.0 null null)))
      (elif (`self.GameStart`)
        (goto _label_2)
        (else
          ;[1 1 1] Tutorial Loop
          (bind _outactors (`GameplayStatics.GetAllActorsOfClass` "/Game/ShatteredMoon/BluePrints/StartGameBttn_BP.StartGameBttn_BP_C"))
          (if (`/Game/ShatteredMoon/BluePrints/StartGameBttn_BP.bttnPressed` (`|GetArrayItem` _outactors))
            (bind _output_get_3 (set `self.bttnHeldTimer` (- (`self.bttnHeldTimer`) DeltaSeconds)))
            (if (<= _output_get_3 0.0)
              (`/Game/VirtualRealityBP/Blueprints/MotionControllerPawn.FadeOut` _vr_camera)
              (`KismetSystemLibrary.Delay` 2.0)
              (`GameplayStatics.PlaySound2D` "/Game/ShatteredMoon/Audio/Tracks/Stand_And_Fight_SYNC_0343_06_Wayne_Dineley_Synctracks.Stand_And_Fight_SYNC_0343_06_Wayne_Dineley_Synctracks" 0.75 1.0 0.0 null null)
              (bind _outactors_2 (`GameplayStatics.GetAllActorsWithTag` "tutorial"))
              (for _array_element _outactors_2
                (if (`self.ActorHasTag` _array_element "Tazer")
                  ;[1 1 1] If Tazer is not held, destroy...
                  (bind _astaser_eagle_bp (cast `/Game/ShatteredMoon/BluePrints/Weapon/TaserEagle_BP` _array_element)
                    (:`then`
                      (if (not (`/Game/ShatteredMoon/BluePrints/Weapon/TaserEagle_BP.held` _astaser_eagle_bp))
                        (`self.K2_DestroyActor` _array_element :!label _label_4)
                        (`KismetSystemLibrary.Delay` 10.0)
                        (`GameplayStatics.PlaySound2D` "/Game/ShatteredMoon/Audio/Voice/OldAudio/ShMoonPuppies.ShMoonPuppies" 1.0 1.0 0.0 null null)))
                    (:`CastFailed`
                      (goto _label_4)))
                  (elif (`self.ActorHasTag` _array_element "BoomSword")
                    ;[1 1 1] If BoomSword is not held. Destroy
                    (bind _asboom_sword_bp (cast `/Game/ShatteredMoon/BluePrints/Weapon/BoomSword_BP` _array_element)
                      (:`then`
                        (if (not (`/Game/ShatteredMoon/BluePrints/Weapon/BoomSword_BP.held` _asboom_sword_bp))
                          (goto _label_4)))
                      (:`CastFailed`
                        (goto _label_4)))
                    (elif (`self.ActorHasTag` _array_element "Fist")
                      ;[1 1 1] If Gauntlet is not held, destroy
                      (bind _asgauntletts_bp (cast `/Game/ShatteredMoon/BluePrints/Weapon/Gauntletts_BP` _array_element)
                        (:`then`
                          (if (not (`/Game/ShatteredMoon/BluePrints/Weapon/Gauntletts_BP.held` _asgauntletts_bp))
                            (goto _label_4)))
                        (:`CastFailed`
                          (goto _label_4)))
                      (else
                        (goto _label_4))))))
              (set `self.GameStart` true)
              (`KismetSystemLibrary.Delay` 2.0)
              (`/Game/VirtualRealityBP/Blueprints/MotionControllerPawn.FadeIn` _vr_camera)
              (`KismetSystemLibrary.Delay` 2.0)
              (`/Game/VirtualRealityBP/Blueprints/MotionControllerPawn.Stop Fade` _vr_camera))
            (else
              (set `self.bttnHeldTimer` 3.0))))))
    (else
      (set `self.playerIsDead` true)
      (goto _label))))

(fn `burst spawn`
  (params (`Enemy Type` :type "Pawn Class Reference") (`Number of Enemies` :type Integer :default 15))
  (bind _spawn_points (`self.spawn points`))
  (bind _defaultsceneroot (`/Game/ShatteredMoon/BluePrints/Enemy/EnemySpawnPoint_BP.DefaultSceneRoot` (`|GetArrayItem` _spawn_points (`KismetMathLibrary.RandomInteger` (`KismetArrayLibrary.Array_Length` _spawn_points)))))
  (for _ (range (+ `Number of Enemies` 1))
    (`AIBlueprintHelperLibrary.SpawnAIFromClass` `Enemy Type` null (`SceneComponent.K2_GetComponentLocation` _defaultsceneroot) (`SceneComponent.K2_GetComponentRotation` _defaultsceneroot))
    (set `self.Enemy Count` (+ (`self.Enemy Count`) 1))
    (if (== `Enemy Type` "/Game/ShatteredMoon/BluePrints/Enemy/Wasp_BP.Wasp_BP_C")
      (bind _output_get (set `self.WaspCounter` (+ (stale _output_get) 1))))))

(fn `Get Number of Enemies`
  (bind _outactors (`GameplayStatics.GetAllActorsOfClass` "/Game/ShatteredMoon/BluePrints/Enemy/Wasp_BP.Wasp_BP_C"))
  (bind _outactors_2 (`GameplayStatics.GetAllActorsOfClass` "/Game/ShatteredMoon/BluePrints/Enemy/Wolf_BP.Wolf_BP_C"))
  (set `self.Enemy Count` (+ (`KismetArrayLibrary.Array_Length` _outactors_2) (`KismetArrayLibrary.Array_Length` _outactors))))

(fn `GetCamera Location`
  (returns (TransformLocation :type "Vector Structure"))
  (bind (_returnvalue_x _returnvalue_y) (`KismetMathLibrary.BreakVector` (`SceneComponent.K2_GetComponentLocation` (`/Game/VirtualRealityBP/Blueprints/MotionControllerPawn.Camera` (`self.VR Camera`)))))
  (return (`KismetMathLibrary.MakeVector` _returnvalue_x _returnvalue_y 100.0)))

(fn `hit player`
  (if (<= (`self.playerCanBeHitTimer`) 0.0)
    (set `self.playerCanBeHitTimer` 1.0)
    (set `self.CanHitPlayer` true))
  (if (`self.CanHitPlayer`)
    (set `self.CanHitPlayer` false)
    (bind _output_get (set `self.playerHealth` (- (stale _output_get) 1)))
    (`GameplayStatics.PlaySound2D` "/Game/ShatteredMoon/Audio/SFX/HumanMaleGrunt.HumanMaleGrunt" 1.0 1.0 0.0 null null)))

(fn `picked up BoomSword`
  (if (not (`self.boomSwordPicked`))
    (`GameplayStatics.PlaySound2D` "/Game/ShatteredMoon/Audio/Voice/PlainBoomSword_Hotton.PlainBoomSword_Hotton" 1.0 1.0 0.0 null null)
    (set `self.boomSwordPicked` true)))

(fn `picked up Gauntlet`
  (if (not (`self.GauntletPicked`))
    (`GameplayStatics.PlaySound2D` "/Game/ShatteredMoon/Audio/Voice/PlainDragonGloves_Hotton.PlainDragonGloves_Hotton" 1.0 1.0 0.0 null null)
    (set `self.GauntletPicked` true)))

(fn `picked up Tazer`
  (if (not (`self.tazerPicked`))
    (`GameplayStatics.PlaySound2D` "/Game/ShatteredMoon/Audio/Voice/PlainTaserEagle_Hotton.PlainTaserEagle_Hotton" 1.0 1.0 0.0 null null)
    (set `self.tazerPicked` true)))

(fn `UserConstructionScript`)
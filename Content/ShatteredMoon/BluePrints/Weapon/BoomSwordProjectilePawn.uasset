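; BoomSwordProjectilePawn is a weapon projectile that damages whatever it hits.
; A Dead flag limits it to one hit, which spawns impact effects, applies damage, deactivates its particle system and destroys it after a short delay.
; Impact effects depend on actor tags: wasps and wolves share a velocity-oriented emitter, land gets sand particles with sound, and other targets get none.
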(event `self.ReceiveBeginPlay`)

(event `self.ReceiveActorBeginOverlap`
  (params (OtherActor :type "Actor Object Reference")))

(event `self.ReceiveHit`
  (params (MyComp :type "PrimitiveComponent Object Reference") (Other :type "Actor Object Reference") (OtherComp :type "PrimitiveComponent Object Reference") (bSelfMoved :type Boolean) (HitLocation :type "Vector Structure") (HitNormal :type "Vector Structure") (NormalImpulse :type "Vector Structure") (Hit :type "HitResult Structure (by ref)"))
  (if (not (`self.dead`))
    (set `self.dead` true)
    (`self.Spawn Impact Particles` Other)
    (`GameplayStatics.ApplyDamage` Other 30.0 null null "/Script/Engine.DamageType")
    (`ActorComponent.Deactivate` (`self.ParticleSystem`))
    (`KismetSystemLibrary.Delay` 1.0)
    (`self.K2_DestroyActor`)))

(fn `Spawn Impact Particles`
  (params (`Object Hit` :type "Actor Object Reference"))
  (bind _returnvalue (`self.K2_GetActorLocation`))
  (if (`self.ActorHasTag` `Object Hit` "Wasp")
    (`GameplayStatics.SpawnEmitterAtLocation` "/Game/ShatteredMoon/Particles/WaspBulletImpact.WaspBulletImpact" _returnvalue (`KismetMathLibrary.Conv_VectorToRotator` (`MovementComponent.Velocity` (`self.ProjectileMovement`))) :!label _label)
    (elif (`self.ActorHasTag` `Object Hit` "enemyWolf")
      (goto _label)
      (elif (`self.ActorHasTag` `Object Hit` "land")
        (`GameplayStatics.PlaySoundAtLocation` "/Game/ShatteredMoon/Audio/SFX/sand_bullet_impact_Gardei.sand_bullet_impact_Gardei" _returnvalue (struct) 0.5 1.0 0.0 null null null)
        (`GameplayStatics.SpawnEmitterAtLocation` "/Game/ShatteredMoon/Particles/sand_bullet_impact.sand_bullet_impact" (+ _returnvalue (0.0 0.0 1.5)))))))

(fn `UserConstructionScript`)
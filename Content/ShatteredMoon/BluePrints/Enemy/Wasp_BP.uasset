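; Wasp enemy that flies toward a point above the camera location supplied by ShatteredMoon_BaseMode, facing the camera.
; While alive, Tick drives procedural wing flapping with clamped pitch, direct location steering, and timed random left or right impulses.
; Damage plays a hit sound and reduces health.
; Death updates GameMode kill and enemy counts, breaks the body parts into physics-simulated pieces, then destroys the actor after a delay.
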(event `self.ReceiveBeginPlay`
  (bind _asshattered_moon_base_mode (cast `/Game/ShatteredMoon/BluePrints/GameMode/ShatteredMoon_BaseMode` (`GameplayStatics.GetGameMode`)))
  (set `self.gameMode` _asshattered_moon_base_mode)
  (set `CharacterMovementComponent.JumpZVelocity` 200.0 (`self.CharacterMovement`))
  (`CharacterMovementComponent.AddImpulse` (`self.CharacterMovement`) (0.0 0.0 50000.0) false))

(event `self.ReceiveAnyDamage`
  (params (Damage :type "Float (single-precision)") (DamageType :type "DamageType Object Reference") (InstigatedBy :type "Controller Object Reference") (DamageCauser :type "Actor Object Reference"))
  (bind _gamemode (`self.gameMode`))
  (bind _wasp_head (`self.wasp_head`))
  (bind _returnvalue (`SceneComponent.K2_GetComponentLocation` (`self.Mesh`)))
  ;[1 1 1] When wasp is hit...
  (if (not (`self.dead`))
    (bind _output_get (set `self.Health` (- (`self.Health`) Damage)))
    (if (<= _output_get 0.0)
      ;;[1 1 1] Kill wasp if health is less than or equal to 0.
      (set `self.dead` true)
      (bind _output_get_2 (set `/Game/ShatteredMoon/BluePrints/GameMode/ShatteredMoon_BaseMode.Enemies Killed` (+ (stale _output_get_2) 1) _gamemode))
      (bind _output_get_3 (set `/Game/ShatteredMoon/BluePrints/GameMode/ShatteredMoon_BaseMode.Enemy Count` (- (stale _output_get_3) 1) _gamemode))
      (`GameplayStatics.SpawnSoundAtLocation` "/Game/ShatteredMoon/Audio/beeHit.beeHit" _returnvalue (struct) 1.0 1.0 0.0 null null)
      (`CharacterMovementComponent.SetMovementMode` (`self.CharacterMovement`) "MOVE_Falling" 0)
      (`SceneComponent.K2_DetachFromComponent` _wasp_head "KeepWorld" "KeepWorld" "KeepWorld" true)
      (`SceneComponent.K2_DetachFromComponent` (`self.wasp_abdomen`) "KeepWorld" "KeepWorld" "KeepWorld" true)
      (`SceneComponent.K2_DetachFromComponent` (`self.wasp_rWing`) "KeepWorld" "KeepWorld" "KeepWorld" true)
      (`SceneComponent.K2_DetachFromComponent` (`self.wasp_lWing`) "KeepWorld" "KeepWorld" "KeepWorld" true)
      (`PrimitiveComponent.SetMassOverrideInKg` _wasp_head "None" 5000.0 true)
      (`PrimitiveComponent.SetMassOverrideInKg` (`self.wasp_abdomen`) "None" 5000.0 true)
      (`PrimitiveComponent.SetMassOverrideInKg` (`self.wasp_rWing`) "None" 5000.0 true)
      (`PrimitiveComponent.SetMassOverrideInKg` (`self.wasp_lWing`) "None" 5000.0 true)
      (`PrimitiveComponent.SetMassOverrideInKg` (`self.wasp_body`) "None" 5000.0 true)
      (`PrimitiveComponent.SetSimulatePhysics` _wasp_head true)
      (`PrimitiveComponent.SetSimulatePhysics` (`self.wasp_abdomen`) true)
      (`PrimitiveComponent.SetSimulatePhysics` (`self.wasp_rWing`) true)
      (`PrimitiveComponent.SetSimulatePhysics` (`self.wasp_lWing`) true)
      (`PrimitiveComponent.SetSimulatePhysics` (`self.wasp_body`) true)
      (`PrimitiveComponent.SetEnableGravity` _wasp_head true)
      (`PrimitiveComponent.SetEnableGravity` (`self.wasp_abdomen`) true)
      (`PrimitiveComponent.SetEnableGravity` (`self.wasp_rWing`) true)
      (`PrimitiveComponent.SetEnableGravity` (`self.wasp_lWing`) true)
      (`PrimitiveComponent.SetEnableGravity` (`self.wasp_body`) true)
      (`KismetSystemLibrary.Delay` 2.0)
      (`self.K2_DestroyActor`)
      (else
        ;;[1 1 1] Play Wounded Wasp Noise
        (`GameplayStatics.SpawnSoundAtLocation` "/Game/ShatteredMoon/Audio/beeHit.beeHit" _returnvalue (struct) 1.0 1.0 0.0 null null)))))

(event `self.ReceiveTick`
  (params (DeltaSeconds :type "Float (single-precision)"))
  (if (not (`self.dead`))
    (`self.flapWings` DeltaSeconds)
    (bind _transformlocation (`/Game/ShatteredMoon/BluePrints/GameMode/ShatteredMoon_BaseMode.GetCamera Location` (`self.gameMode`)))
    (`self.flyTo` _transformlocation DeltaSeconds)))

(fn `flapWings`
  (params (deltaTime :type "Float (double-precision)"))
  (bind _wasp_rwing (`self.wasp_rWing`))
  (bind _wasp_lwing (`self.wasp_lWing`))
  (bind _wasp_rwing_2 (`self.wasp_rWing`))
  (bind _wasp_lwing_2 (`self.wasp_lWing`))
  (bind _wingflaprate (`self.wingFlapRate`))
  (bind _flap_timer (`self.flap timer`))
  (bind (_relativerotation_roll _relativerotation_pitch) (`KismetMathLibrary.BreakRotator` (`SceneComponent.RelativeRotation` _wasp_lwing_2)))
  (bind (_relativerotation_roll_2 _relativerotation_pitch_2) (`KismetMathLibrary.BreakRotator` (`SceneComponent.RelativeRotation` _wasp_rwing)))
  (bind (_relativerotation_roll_3 _relativerotation_pitch_3) (`KismetMathLibrary.BreakRotator` (`SceneComponent.RelativeRotation` _wasp_lwing)))
  (bind (_relativerotation_roll_4 _relativerotation_pitch_4) (`KismetMathLibrary.BreakRotator` (`SceneComponent.RelativeRotation` _wasp_rwing_2)))
  (if (`self.up`)
    (set `self.wingFlapRate` 15.0)
    (else
      (set `self.wingFlapRate` -15.0)))
  ;[1 1 1] Wing Rotation Restriction - If the wing goes to far, this code will bring the wing back in.
  (if (`self.up`)
    (if (not (<= _relativerotation_pitch_3 15.0))
      (`SceneComponent.K2_SetRelativeRotation` _wasp_lwing (struct :`Pitch` 15.0) false false)
      (set `self.clamped L Wing` true))
    (if (<= _relativerotation_pitch_4 -15.0)
      (`SceneComponent.K2_SetRelativeRotation` _wasp_rwing_2 (struct :`Pitch` -15.0) false false)
      (set `self.clamped R Wing` true))
    (else
      (if (<= _relativerotation_pitch_2 15.0)
        (`SceneComponent.K2_SetRelativeRotation` _wasp_rwing (struct :`Pitch` 15.0) false false)
        (set `self.clamped R Wing` true))
      (if (<= _relativerotation_pitch -15.0)
        (`SceneComponent.K2_SetRelativeRotation` _wasp_lwing_2 (struct :`Pitch` -15.0) false false)
        (set `self.clamped L Wing` true))))
  (if (not (`self.clamped L Wing`))
    (`SceneComponent.K2_AddRelativeRotation` (`self.wasp_lWing`) (`KismetMathLibrary.MakeRotator` 0.0 _wingflaprate) false false))
  (if (not (`self.clamped R Wing`))
    (`SceneComponent.K2_AddRelativeRotation` (`self.wasp_rWing`) (`KismetMathLibrary.MakeRotator` 0.0 (* _wingflaprate -1.0)) false false))
  (if (<= _flap_timer 0.0)
    (set `self.flap timer` 0.01)
    (if (`self.up`)
      (set `self.up` false)
      (else
        (set `self.up` true)))
    (set `self.clamped R Wing` false)
    (set `self.clamped L Wing` false)
    (else
      (set `self.flap timer` (- _flap_timer (`local.deltaTime`))))))

(fn `flyTo`
  (params (target :type "Vector Structure") (deltaTime :type "Float (double-precision)"))
  (bind _returnvalue (`self.K2_GetActorLocation`))
  (bind _returnvalue_2 (+ target (0.0 0.0 300.0)))
  (if (>= (`KismetMathLibrary.VSizeXY` (+ _returnvalue _returnvalue_2)) 600.0)
    (`self.K2_SetActorLocation` (+ _returnvalue (* (* (- _returnvalue_2 _returnvalue) deltaTime) (* (`self.speed`) (`self.SlowDown`))))))
  (`self.K2_SetActorRotation` (`KismetMathLibrary.FindLookAtRotation` _returnvalue target))
  (`self.sideStep` deltaTime))

(fn `sideStep`
  (params (deltaTime :type "Float (double-precision)"))
  (bind _returnvalue (`self.K2_GetActorRotation`))
  (bind _returnvalue_2 (`self.K2_GetActorRotation`))
  (bind _step_timer (`self.step timer`))
  (bind _charactermovement (`self.CharacterMovement`))
  (if (<= _step_timer 0.0)
    (set `self.step timer` 0.5)
    (if (`KismetMathLibrary.RandomBool`)
      (`CharacterMovementComponent.AddImpulse` _charactermovement (+ (`self.GetVelocity`) (+ (* (`KismetMathLibrary.GetRightVector` _returnvalue_2) -5000.0) (* (`KismetMathLibrary.GetForwardVector` _returnvalue_2) 1.0))) false)
      (else
        (`CharacterMovementComponent.AddImpulse` _charactermovement (+ (`self.GetVelocity`) (+ (* (`KismetMathLibrary.GetRightVector` _returnvalue) 5000.0) (* (`KismetMathLibrary.GetForwardVector` _returnvalue) 1.0))) false)))
    (else
      (set `self.step timer` (- _step_timer deltaTime)))))

(fn `UserConstructionScript`)
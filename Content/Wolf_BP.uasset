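; Wolf enemy for a VR game that chases the player's headset, using the camera location from ShatteredMoon_BaseMode.
; Tick reissues AIMoveTo and runs a bounce timer that jumps with random left or right impulses.
; DodgeCheck, not called here, arms a stronger sideways dodge on a cooldown; the close-range distance check has no effect.
; Damage plays a yelp, and death updates the GameMode's kill and enemy counts before destroying the wolf.
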(event `self.ReceiveBeginPlay`
  ;[1 1 1] On game start... Get Game mode. Needed to get location of VR headset.
  (bind _asshattered_moon_base_mode (cast `/Game/ShatteredMoon/BluePrints/ShatteredMoon_BaseMode` (`GameplayStatics.GetGameMode`)))
  (set `self.gameMode` _asshattered_moon_base_mode)
  (set `CharacterMovementComponent.JumpZVelocity` 200.0 (`self.CharacterMovement`)))

(event `self.ReceiveAnyDamage`
  (params (Damage :type "Float (single-precision)") (DamageType :type "DamageType Object Reference") (InstigatedBy :type "Controller Object Reference") (DamageCauser :type "Actor Object Reference"))
  (bind _gamemode (`self.gameMode`))
  (bind _returnvalue (`SceneComponent.K2_GetComponentLocation` (`self.Mesh`)))
  ;[1 1 1] When wolf is hit...
  (bind _output_get (set `self.Health` (- (`self.Health`) Damage)))
  (if (<= _output_get 0.0)
    ;;[1 1 1] Kill wolf if health is less than or equal to 0.
    (bind _output_get_2 (set `/Game/ShatteredMoon/BluePrints/ShatteredMoon_BaseMode.Enemies Killed` (+ (stale _output_get_2) 1) _gamemode))
    (bind _output_get_3 (set `/Game/ShatteredMoon/BluePrints/ShatteredMoon_BaseMode.Enemy Count` (- (stale _output_get_3) 1) _gamemode))
    (`GameplayStatics.SpawnSoundAtLocation` "/Game/ShatteredMoon/Music_SFX/SFX/163280__tobiaskosmos__dogyelp.163280__tobiaskosmos__dogyelp" _returnvalue (struct) 1.0 1.0 0.0 null null)
    (`self.K2_DestroyActor`)
    (else
      ;;[1 1 1] Play Wounded dog noise
      (`GameplayStatics.SpawnSoundAtLocation` "/Game/ShatteredMoon/Music_SFX/SFX/163280__tobiaskosmos__dogyelp.163280__tobiaskosmos__dogyelp" _returnvalue (struct) 1.0 1.0 0.0 null null))))

(event `self.ReceiveTick`
  (params (DeltaSeconds :type "Float (single-precision)"))
  (bind _returnvalue (`self.K2_GetActorRotation`))
  (bind _returnvalue_2 (`self.K2_GetActorRotation`))
  (bind _bouncetimer (`self.bounceTimer`))
  (bind _stopbouncetimer (`self.stopBounceTimer`))
  ;[1 1 1] AI Logic
  (bind _output_get (set `self.dodgeTimer` (- (stale _output_get) DeltaSeconds)))
  (bind _transformlocation (`/Game/ShatteredMoon/BluePrints/ShatteredMoon_BaseMode.GetCamera Location` (`self.gameMode`)))
  (bind (_returnvalue_x _returnvalue_y) (`KismetMathLibrary.BreakVector` (- _transformlocation (`self.K2_GetActorLocation`))))
  (if (< (`KismetMathLibrary.VSize` (`KismetMathLibrary.MakeVector` _returnvalue_x _returnvalue_y)) 300.0)
    _
    (else
      _))
  ;;[1 1 1] If not too close, run towards player headset.
  (`|AIMoveTo` self _transformlocation null 1.0
    (:`then`
      (bind _output_get_2 (set `self.bounceTimer` (- _bouncetimer DeltaSeconds)))
      (if (<= _output_get_2 0.0)
        (`self.Jump`)
        (set `self.bounceTimer` (`self.bounceInterval`))
        (`KismetSystemLibrary.Delay` 0.05)
        (if (`self.canDodge`)
          (`self.ExecuteDodge`)
          (elif (`KismetMathLibrary.RandomBool`)
            (`CharacterMovementComponent.AddImpulse` (`self.CharacterMovement`) (+ (`self.GetVelocity`) (+ (* (`KismetMathLibrary.GetRightVector` _returnvalue_2) -10000.0) (* (`KismetMathLibrary.GetForwardVector` _returnvalue_2) 5000.0))) false) ; bounce left
            (else
              (`CharacterMovementComponent.AddImpulse` (`self.CharacterMovement`) (+ (`self.GetVelocity`) (+ (* (`KismetMathLibrary.GetRightVector` _returnvalue) 10000.0) (* (`KismetMathLibrary.GetForwardVector` _returnvalue) 5000.0))) false) ; bounce right
            )))
        (elif (<= _stopbouncetimer 0.0)
          (`self.StopJumping`)
          (set `self.stopBounceTimer` (/ _bouncetimer 2.0))
          (else
            (set `self.stopBounceTimer` (- _stopbouncetimer DeltaSeconds))))))))

(fn `DodgeCheck`
  (if (<= (stale _output_get) 0.0)
    (bind _output_get (set `self.dodgeTimer` 2.0))
    (set `self.canDodge` true)))

(fn `ExecuteDodge`
  (bind _returnvalue (`self.K2_GetActorRotation`))
  (bind _returnvalue_2 (`self.K2_GetActorRotation`))
  (set `self.canDodge` false)
  (if (`KismetMathLibrary.RandomBool`)
    (`CharacterMovementComponent.AddImpulse` (`self.CharacterMovement`) (+ (`self.GetVelocity`) (+ (* (`KismetMathLibrary.GetRightVector` _returnvalue_2) -50000.0) (* (`KismetMathLibrary.GetForwardVector` _returnvalue_2) 5000.0))) false) ; bounce left
    (else
      (`CharacterMovementComponent.AddImpulse` (`self.CharacterMovement`) (+ (`self.GetVelocity`) (+ (* (`KismetMathLibrary.GetRightVector` _returnvalue) 50000.0) (* (`KismetMathLibrary.GetForwardVector` _returnvalue) 5000.0))) false) ; bounce right
    )))

(fn `UserConstructionScript`
  (bind _outactors (`GameplayStatics.GetAllActorsOfClass` "/Game/VirtualRealityBP/Blueprints/MotionControllerPawn.MotionControllerPawn_C"))
  (set `self.target` (`|GetArrayItem` _outactors)))
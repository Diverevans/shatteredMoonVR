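; Gauntlet weapon that a motion controller picks up, giving the player a shotgun blast and a melee strike.
; Pickup attaches it to the controller and notifies the game mode; Drop restores physics and also runs when the player dies.
; Firing, limited by a Tick-driven cooldown, repeatedly spawns randomly spread projectile pawns and muzzle effects from three barrels.
; While held, its hit box damages enemy-tagged actors, and both attacks rumble the controller.
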(event `self.ReceiveBeginPlay`
  (bind _asshattered_moon_base_mode (cast `/Game/ShatteredMoon/BluePrints/GameMode/ShatteredMoon_BaseMode` (`GameplayStatics.GetGameMode`)))
  (set `self.gameMode` _asshattered_moon_base_mode))

(event `/Game/VirtualRealityBP/Blueprints/PickupActorInterface.Pickup`
  (params (AttachTo :type "SceneComponent Object Reference") (Controller :type "/Game/VirtualRealityBP/Blueprints/BP_MotionController Object Reference"))
  (set `self.Controller` Controller)
  (`PrimitiveComponent.SetSimulatePhysics` (`self.StaticMeshComponent`) false)
  (`SceneComponent.K2_AttachToComponent` (`self.K2_GetRootComponent`) AttachTo "None" "SnapToTarget" "SnapToTarget" "KeepWorld" false)
  (set `self.held` true)
  (`/Game/ShatteredMoon/BluePrints/GameMode/ShatteredMoon_BaseMode.picked up Gauntlet` (`self.GameMode`)) ; triggers the audio queue for picking up the guantlet for first time.
)

(event `/Game/VirtualRealityBP/Blueprints/PickupActorInterface.Drop`
  (`PrimitiveComponent.SetSimulatePhysics` (`self.StaticMeshComponent`) true)
  (`self.K2_DetachFromActor` "KeepWorld" "KeepWorld" "KeepWorld")
  (set `self.held` false))

(event `self.ReceiveTick`
  (params (DeltaSeconds :type "Float (single-precision)"))
  (if (`self.held`)
    (bind _output_get (set `self.shotDelayTimer` (- (stale `self.ReceiveTick` _output_get) DeltaSeconds)))
    (if (`/Game/ShatteredMoon/BluePrints/GameMode/ShatteredMoon_BaseMode.playerIsDead` (`self.GameMode`))
      (`/Game/VirtualRealityBP/Blueprints/PickupActorInterface.Drop`))))

(event `/Game/VirtualRealityBP/Blueprints/PickupActorInterface.FireWeapon`
  (if (and (`self.held`) (<= (stale `self.ReceiveTick` _output_get) 0.0))
    (set `self.shotDelayTimer` 1.0)
    (`GameplayStatics.PlaySoundAtLocation` "/Game/ShatteredMoon/Audio/SFX/GunShots/shotgun_Grab_2_2_GardeiEvans_clickboost.shotgun_Grab_2_2_GardeiEvans_clickboost" (`SceneComponent.K2_GetComponentLocation` (`self.barrel2`)) (struct) 1.0 1.0 0.0 null null null)
    (for _ (range 13)
      (`self.Fire Barrel` (`self.barrel1`))
      (`self.Fire Barrel` (`self.barrel2`))
      (`self.Fire Barrel` (`self.barrel3`)))
    (`/Game/VirtualRealityBP/Blueprints/BP_MotionController.RumbleController` (`self.Controller`) 1.0)))

(event `self.MeleeHitBox.OnComponentBeginOverlap`
  (params (OverlappedComponent :type "PrimitiveComponent Object Reference") (OtherActor :type "Actor Object Reference") (OtherComp :type "PrimitiveComponent Object Reference") (OtherBodyIndex :type Integer) (bFromSweep :type Boolean) (SweepResult :type "HitResult Structure (by ref)"))
  (bind _controller (`self.Controller`))
  (if (and (`self.held`) (`self.ActorHasTag` OtherActor "enemy"))
    (`GameplayStatics.PlaySoundAtLocation` "/Game/ShatteredMoon/Audio/SFX/77611__joelaudio__sfx-attack-sword-001.77611__joelaudio__sfx-attack-sword-001" (`self.K2_GetActorLocation` OtherActor) (struct) 1.0 1.0 0.0 null null null)
    (`GameplayStatics.ApplyDamage` OtherActor (`self.MeleeDamageAmount`))
    (`/Engine/EditorBlueprintResources/StandardMacros.IsValid` _controller
      (:`Is Valid`
        (`/Game/VirtualRealityBP/Blueprints/BP_MotionController.RumbleController` _controller 1.0)))))

(fn `Fire Barrel`
  (params (barrel :type "SceneComponent Object Reference"))
  (bind (_returnvalue_roll _returnvalue_pitch _returnvalue_yaw) (`KismetMathLibrary.BreakRotator` (`SceneComponent.K2_GetComponentRotation` barrel)))
  (bind _returnvalue (`SceneComponent.K2_GetComponentLocation` barrel))
  (bind _returnvalue_2 (`KismetMathLibrary.MakeRotator` _returnvalue_roll (+ _returnvalue_pitch (`KismetMathLibrary.RandomFloatInRange` -5.0 5.0)) (+ _returnvalue_yaw (`KismetMathLibrary.RandomFloatInRange` -5.0 5.0))))
  (if true
    (`GameplayStatics.SpawnEmitterAtLocation` "/Game/ShatteredMoon/Particles/GauntletShotBlast.GauntletShotBlast" _returnvalue (`SceneComponent.K2_GetComponentRotation` barrel))
    (`|SpawnActorFromClass` "/Game/ShatteredMoon/BluePrints/Weapon/GauntletProjectilePawn.GauntletProjectilePawn_C" (`KismetMathLibrary.MakeTransform` (+ _returnvalue (`KismetMathLibrary.GreaterGreater_VectorRotator` (`self.gunOffset`) _returnvalue_2)) _returnvalue_2) "Undefined" "OverrideRootScale" null null)))

(fn `UserConstructionScript`)
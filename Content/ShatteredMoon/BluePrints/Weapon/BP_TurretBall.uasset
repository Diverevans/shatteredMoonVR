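; Throwable turret ball, picked up and dropped through the motion controller, that deploys a turret where it lands.
; While held, Tick measures button depression to prime the ball with sound and particles, counting presses for spam warnings and a SwolWolf easter egg.
; Once released and primed, a sphere overlap detects the Landscape, plays a deploy effect, then spawns the turret, or SwolWolf if unlocked, and destroys the ball.
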(event `self.ReceiveTick`
  (params (DeltaSeconds :type "Float (single-precision)"))
  (bind _returnvalue (`self.K2_GetActorLocation`))
  (bind _returnvalue_2 (+ _returnvalue 1))
  (bind _returnvalue_3 (`SceneComponent.K2_GetComponentLocation` (`self.SpringArm`)))
  (if (`self.Held`)
    ;[1 1 1] If Button pressed while held, prime turret and play audio queue
    (bind _output_get (set `self.ButtonDistance` (`KismetMathLibrary.VSize` (- _returnvalue_3 (`SceneComponent.K2_GetComponentLocation` (`self.Top of Button`))))))
    (if (<= _output_get 0.25)
      (if (not (`self.BttnPressed`))
        (`GameplayStatics.PlaySoundAtLocation` "/Game/ShatteredMoon/Audio/SFX/click_Gardei.click_Gardei" _returnvalue_3 (struct) 1.0 1.0 0.0 null null null)
        (set `self.Primed` true)
        (set `self.BttnPressed` true) ; prevents audio from looping while button is held down
        (`ActorComponent.Activate` (`self.ParticleSystem`) false)
        (bind _output_get_2 (set `self.pressCounter` (+ (stale _output_get_2) 1)))
        (if (== _output_get_2 5)
          (`GameplayStatics.PlaySound2D` null 1.0 1.0 0.0 null null) ; stop spamming the button que
          (elif (>= _output_get_2 10)
            (set `self.SWOL` true)
            (`GameplayStatics.PlaySound2D` null 1.0 1.0 0.0 null null) ; swolwolf audio tease
            (`KismetSystemLibrary.Delay` 1.0)
            (`GameplayStatics.PlaySound2D` null 1.0 1.0 0.0 null null) ; did it just say swolwolf?
          )))
      (else
        (set `self.BttnPressed` false)))
    (else
      ;[1 1 1] If not held and turret is primed...
      (if (and (!= (`self.Held`) true) (`self.Primed`))
        (bind (_outactors _returnvalue_4) (`KismetSystemLibrary.SphereOverlapActors` _returnvalue 5.0 (`|MakeArray` "ObjectTypeQuery1" :!type "EObjectTypeQuery Enum") "/Script/Landscape.Landscape"))
        (if _returnvalue_4
          ;[1 1 1] Deploy Turret and kill turret ball
          (if (not (`self.Deploying`))
            (`GameplayStatics.SpawnEmitterAtLocation` "/Game/ShatteredMoon/Particles/TurretDeploy.TurretDeploy" _returnvalue_2)
            (set `self.Deploying` true)
            (`PrimitiveComponent.SetSimulatePhysics` (`self.StaticMeshComponent`) false)
            (`KismetSystemLibrary.Delay` 0.5)
            (if (`self.SWOL`)
              (`AIBlueprintHelperLibrary.SpawnAIFromClass` "/Game/ShatteredMoon/BluePrints/Weapon/SwolWolf/SwolWolf_BP.SwolWolf_BP_C" null (`KismetMathLibrary.MakeVector` (.x _returnvalue_2) (.y _returnvalue_2) 150.0))
              (else
                (`|SpawnActorFromClass` "/Game/ShatteredMoon/BluePrints/Weapon/Turret_Blueprint.Turret_Blueprint_C" (`KismetMathLibrary.Conv_VectorToTransform` _returnvalue_2) "Undefined" "OverrideRootScale" null null)))
            (`self.K2_DestroyActor`)))))))

(event `/Game/VirtualRealityBP/Blueprints/PickupActorInterface.Pickup`
  (params (AttachTo :type "SceneComponent Object Reference") (Controller :type "/Game/VirtualRealityBP/Blueprints/BP_MotionController Object Reference"))
  (`PrimitiveComponent.SetSimulatePhysics` (`self.StaticMeshComponent`) false)
  (`SceneComponent.K2_AttachToComponent` (`self.K2_GetRootComponent`) AttachTo "None" "KeepWorld" "KeepWorld" "KeepWorld" false)
  (set `self.Held` true))

(event `/Game/VirtualRealityBP/Blueprints/PickupActorInterface.Drop`
  (`PrimitiveComponent.SetSimulatePhysics` (`self.StaticMeshComponent`) true)
  (`self.K2_DetachFromActor` "KeepWorld" "KeepWorld" "KeepWorld")
  (set `self.Held` false))

(fn `UserConstructionScript`)
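; StartGameBttn_BP is a physical button, named for starting the game, that plays a click sound when pressed.
; Each Tick it measures the distance between the SpringArm and TopOfBttn components, treating a very small gap as a press.
; A BttnPressed flag latches so the click fires once per press, resetting when the gap widens.
; No game-start logic is wired here, only press detection and audio feedback.
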(event `self.ReceiveTick`
  (params (DeltaSeconds :type "Float (single-precision)"))
  (bind _returnvalue (`SceneComponent.K2_GetComponentLocation` (`self.SpringArm`)))
  (bind _output_get (set `self.bttnDistance` (`KismetMathLibrary.VSize` (- _returnvalue (`SceneComponent.K2_GetComponentLocation` (`self.topOfBttn`))))))
  (if (<= _output_get 0.4)
    (if (not (`self.bttnPressed`))
      (`GameplayStatics.PlaySoundAtLocation` "/Game/ShatteredMoon/Audio/sfx_click.sfx_click" _returnvalue (struct) 1.0 1.0 0.0 null null null)
      (set `self.bttnPressed` true))
    (else
      (set `self.bttnPressed` false))))

(fn `UserConstructionScript`)
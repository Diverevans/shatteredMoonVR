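; EnemySpawnPoint_BP is an enemy spawn point that spawns a Wolf_BP at its root component's transform.
; The SpawnEnemy event spawns one wolf per call whenever MaxEnemies is above zero, without tracking a spawned count.
; Random selection from EnemyList and random placement inside SpawnVolume exist only as unconnected nodes, so neither affects spawning.
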(event `SpawnEnemy`
  (if (< 0 (`self.MaxEnemies`))
    (`|SpawnActorFromClass` "/Game/ShatteredMoon/BluePrints/Enemy/Wolf_BP.Wolf_BP_C" (`SceneComponent.K2_GetComponentToWorld` (`self.DefaultSceneRoot`)) "Undefined" "OverrideRootScale" null null)))

(fn `UserConstructionScript`)
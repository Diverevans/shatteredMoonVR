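; BoomSword is a motion-controller held weapon that works as both a melee sword and a projectile launcher.
; Pickup snaps it to the controller and disables physics, while Drop detaches it and restores physics.
; Its hit box damages actors tagged "enemy", and FireWeapon spawns a projectile pawn from the barrel, both with sound and controller rumble.
; An explosive line-trace shot remains in the graph but is disconnected.
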(event `self.MeleeHitBox.OnComponentBeginOverlap`
  (params (OverlappedComponent :type "PrimitiveComponent Object Reference") (OtherActor :type "Actor Object Reference") (OtherComp :type "PrimitiveComponent Object Reference") (OtherBodyIndex :type Integer) (bFromSweep :type Boolean) (SweepResult :type "HitResult Structure (by ref)"))
  (bind _controller (`self.Controller`))
  (if (`self.ActorHasTag` OtherActor "enemy")
    (`GameplayStatics.PlaySoundAtLocation` "/Game/ShatteredMoon/Music_SFX/SFX/77611__joelaudio__sfx-attack-sword-001.77611__joelaudio__sfx-attack-sword-001" (`self.K2_GetActorLocation` OtherActor) (struct) 1.0 1.0 0.0 null null null)
    (`GameplayStatics.ApplyDamage` OtherActor (`self.MeleeDamageAmount`) null null "/Script/Engine.DamageType")
    (`/Engine/EditorBlueprintResources/StandardMacros.IsValid` _controller
      (:`Is Valid`
        (`/Game/VirtualRealityBP/Blueprints/BP_MotionController.RumbleController` _controller 1.0)))))

(event `/Game/VirtualRealityBP/Blueprints/PickupActorInterface.Pickup`
  (params (AttachTo :type "SceneComponent Object Reference") (Controller :type "/Game/VirtualRealityBP/Blueprints/BP_MotionController Object Reference"))
  (set `self.Controller` Controller)
  (`PrimitiveComponent.SetSimulatePhysics` (`self.StaticMeshComponent`) false)
  (`SceneComponent.K2_AttachToComponent` (`self.K2_GetRootComponent`) AttachTo "None" "SnapToTarget" "SnapToTarget" "KeepWorld" false))

(event `/Game/VirtualRealityBP/Blueprints/PickupActorInterface.Drop`
  (`PrimitiveComponent.SetSimulatePhysics` (`self.StaticMeshComponent`) true)
  (`self.K2_DetachFromActor` "KeepWorld" "KeepWorld" "KeepWorld"))

(event `/Game/VirtualRealityBP/Blueprints/PickupActorInterface.FireWeapon`
  (bind _barrel (`self.Barrel`))
  (bind (_returnvalue_roll _returnvalue_pitch _returnvalue_yaw) (`KismetMathLibrary.BreakRotator` (`SceneComponent.K2_GetComponentRotation` _barrel)))
  (bind _returnvalue (`KismetMathLibrary.MakeRotator` _returnvalue_roll _returnvalue_pitch _returnvalue_yaw))
  (`GameplayStatics.PlaySoundAtLocation` "/Game/ShatteredMoon/Audio/ar_556cal_Grab.ar_556cal_Grab" (`SceneComponent.K2_GetComponentLocation` (`self.Barrel`)) (struct) 1.0 1.0 0.0 null null null)
  (if true
    (`|SpawnActorFromClass` "/Game/ShatteredMoon/BluePrints/Weapon/BoomSwordProjectilePawn.BoomSwordProjectilePawn_C" (`KismetMathLibrary.MakeTransform` (+ (`SceneComponent.K2_GetComponentLocation` _barrel) (`KismetMathLibrary.GreaterGreater_VectorRotator` (`self.gunOffset`) _returnvalue)) _returnvalue) "Undefined" "OverrideRootScale" null null)
    (`/Game/VirtualRealityBP/Blueprints/BP_MotionController.RumbleController` (`self.Controller`) 1.0)))

(event `self.ReceiveTick`
  (params (DeltaSeconds :type "Float (single-precision)")))

(fn `UserConstructionScript`)
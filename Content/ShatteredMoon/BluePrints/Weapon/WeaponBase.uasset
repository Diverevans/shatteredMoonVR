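; WeaponBase is a base weapon Blueprint for a hand-held weapon that supports both shooting and melee.
; The left or right trigger, matched to its Hand, calls ShootGun, which traces from the Barrel, spawns an explosion and damages the hit actor.
; Each shot increments Ammo rather than decrementing it, and empty ammo runs a 2D sound call instead.
; MeleeHitBox overlaps apply separate melee damage.
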(event `self.MeleeHitBox.OnComponentHit`
  (params (HitComponent :type "PrimitiveComponent Object Reference") (OtherActor :type "Actor Object Reference") (OtherComp :type "PrimitiveComponent Object Reference") (NormalImpulse :type "Vector Structure") (Hit :type "HitResult Structure (by ref)")))

(event `InputAction|LeftTrigger` :consume false
  (params (Key :type "Key Structure"))
  (:`Pressed`
    (if (`|EnumEquality` (`self.Hand`) "Left")
      (`self.ShootGun` :!label _label))))

(event `self.MeleeHitBox.OnComponentBeginOverlap`
  (params (OverlappedComponent :type "PrimitiveComponent Object Reference") (OtherActor :type "Actor Object Reference") (OtherComp :type "PrimitiveComponent Object Reference") (OtherBodyIndex :type Integer) (bFromSweep :type Boolean) (SweepResult :type "HitResult Structure (by ref)"))
  (`GameplayStatics.ApplyDamage` OtherActor (`self.MeleeDamageAmount`)))

(event `InputAction|RightTrigger` :consume false
  (params (Key :type "Key Structure"))
  (:`Pressed`
    (if (`|EnumEquality` (`self.Hand`) "Right")
      (goto _label))))

(fn `ShootGun`
  (bind _returnvalue (`SceneComponent.K2_GetComponentLocation` (`self.Barrel`)))
  (if (<= (`self.Ammo`) 0)
    (`GameplayStatics.PlaySound2D` "/Game/ShatteredMoon/Music_SFX/debugAudio/False.False" 1.0 1.0 0.0 null null)
    (else
      (bind _outhit (`KismetSystemLibrary.LineTraceSingle` :`Start` _returnvalue :`End` (+ _returnvalue (* (`SceneComponent.GetForwardVector` (`self.Barrel`)) 99999999)) :`TraceChannel` "TraceTypeQuery1" :`DrawDebugType` "ForDuration"))
      (bind (_bblockinghit _binitialoverlap _time _distance _location _impactpoint _normal _impactnormal _physmat _hitactor) (`GameplayStatics.BreakHitResult` _outhit))
      (`GameplayStatics.SpawnEmitterAtLocation` "/Game/StarterContent/Particles/P_Explosion.P_Explosion" _location)
      (`GameplayStatics.ApplyDamage` _hitactor (`self.RangeDamageAmount`))
      (set `self.Ammo` (+ (`self.Ammo`) 1)))))

(fn `UserConstructionScript`
  (`parent.UserConstructionScript`))
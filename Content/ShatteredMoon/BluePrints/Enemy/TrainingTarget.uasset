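; Training target actor that topples when damage drains its Health and stands back up after a short delay.
; AnyDamage subtracts from Health, and Tick calls FallDown at zero or counts down StandTimer before calling StandUp.
; Both functions RInterp the root's world rotation to fixed poses, resetting Health and the timer when the pose is reached.
; Downed and GettingUp flags track its state.
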(event `self.ReceiveAnyDamage`
  (params (Damage :type "Float (single-precision)") (DamageType :type "DamageType Object Reference") (InstigatedBy :type "Controller Object Reference") (DamageCauser :type "Actor Object Reference"))
  (set `self.health` (- (`self.health`) Damage)))

(event `self.ReceiveTick`
  (params (DeltaSeconds :type "Float (single-precision)"))
  (bind _stand_timer (`self.stand timer`))
  (if (or (`self.downed`) (`self.getting up`))
    (if (<= (`self.health`) 0.0)
      (`self.fallDown` DeltaSeconds :!label _label)
      (elif (<= _stand_timer 0.0)
        (`self.standUp` DeltaSeconds)
        (else
          (set `self.stand timer` (- _stand_timer DeltaSeconds)))))
    (elif (<= (`self.health`) 0.0)
      (goto _label))))

(fn `fallDown`
  (params (DeltaTime :type "Float (double-precision)"))
  (bind _defaultsceneroot (`self.DefaultSceneRoot`))
  (bind _returnvalue (`KismetMathLibrary.RInterpTo` (`SceneComponent.K2_GetComponentRotation` _defaultsceneroot) (struct) DeltaTime 10.0))
  (set `self.getting up` false)
  (`SceneComponent.K2_SetWorldRotation` _defaultsceneroot _returnvalue false false)
  (if (== _returnvalue (struct) :`ErrorTolerance` 0.001)
    (set `self.downed` true)
    (set `self.stand timer` 5.0)
    (set `self.health` 1.0)))

(fn `standUp`
  (params (deltaTime :type "Float (double-precision)"))
  (bind _defaultsceneroot (`self.DefaultSceneRoot`))
  (bind _returnvalue (`KismetMathLibrary.RInterpTo` (`SceneComponent.K2_GetComponentRotation` _defaultsceneroot) (struct :`Pitch` 90.0) deltaTime 5.0))
  (set `self.getting up` true)
  (`SceneComponent.K2_SetWorldRotation` _defaultsceneroot _returnvalue false false)
  (if (== _returnvalue (struct :`Pitch` 90.0) :`ErrorTolerance` 0.001)
    (set `self.downed` false)
    (set `self.stand timer` 5.0)
    (set `self.health` 1.0)))

(fn `UserConstructionScript`)
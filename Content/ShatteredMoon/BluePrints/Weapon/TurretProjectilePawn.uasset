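; Homing turret projectile pawn that deals radial explosion damage on its first overlap, then destroys itself.
; Tick turns it toward Target and recomputes its local velocity from its speed.
; Without a Target, it veers toward a random point picked at construction, detonates after a short random delay, then cleans up.
; SpawnImpactParticles picks effects by actor tag: bullet impact for Wasp and enemyWolf, sand with sound for land.
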(event `self.ReceiveActorBeginOverlap`
  (params (OtherActor :type "Actor Object Reference"))
  (if (not (`self.detonated`))
    (set `self.detonated` true)
    (`self.Spawn Impact Particles` OtherActor)
    (`GameplayStatics.ApplyRadialDamageWithFalloff` :`BaseDamage` 10.0 :`MinimumDamage` 10.0 :`Origin` (`self.K2_GetActorLocation` self) :`DamageInnerRadius` 100.0 :`DamageOuterRadius` 100.0 :`DamageFalloff` 0.75 :`DamageTypeClass` "/Game/ShatteredMoon/BluePrints/ExplosionDamage.ExplosionDamage_C" :`DamageCauser` null :`InstigatedByController` null :`DamagePreventionChannel` "ECC_WorldStatic")
    (`self.K2_DestroyActor`)))

(event `self.ReceiveTick`
  (params (DeltaSeconds :type "Float (single-precision)"))
  (bind (_returnvalue_roll _returnvalue_pitch) (`KismetMathLibrary.BreakRotator` (`self.K2_GetActorRotation`)))
  (bind (_returnvalue_roll_2 _returnvalue_pitch_2) (`KismetMathLibrary.BreakRotator` (`self.K2_GetActorRotation`)))
  (bind _target (`self.target`))
  (bind _projectilemovement (`self.ProjectileMovement`))
  (`/Engine/EditorBlueprintResources/StandardMacros.IsValid` _target
    (:`Is Valid`
      (`self.K2_SetActorRotation` (`KismetMathLibrary.RInterpTo` (`self.K2_GetActorRotation`) (`KismetMathLibrary.FindLookAtRotation` (`self.K2_GetActorLocation`) (`self.K2_GetActorLocation` _target)) DeltaSeconds 10000.0))
      (`ProjectileMovementComponent.SetVelocityInLocalSpace` _projectilemovement (* (`KismetMathLibrary.CreateVectorFromYawPitch` _returnvalue_roll _returnvalue_pitch (+ (`KismetMathLibrary.VSize` (`self.GetVelocity`)) 5000.0)) 1.1)))
    (:`Is Not Valid`
      (`self.K2_SetActorRotation` (`KismetMathLibrary.RInterpTo` (`self.K2_GetActorRotation`) (`KismetMathLibrary.FindLookAtRotation` (`self.K2_GetActorLocation`) (`self.randomTarget`)) DeltaSeconds 0.5))
      (`ProjectileMovementComponent.SetVelocityInLocalSpace` _projectilemovement (* (`KismetMathLibrary.CreateVectorFromYawPitch` _returnvalue_roll_2 _returnvalue_pitch_2 (+ (`KismetMathLibrary.VSize` (`self.GetVelocity`)) 5000.0)) 0.9))
      (`KismetSystemLibrary.Delay` (`KismetMathLibrary.RandomFloatInRange` 0.25 1.0))
      (if (`self.detonated`)
        (`KismetSystemLibrary.Delay` 3.0)
        (`self.K2_DestroyActor`)
        (else
          (set `self.detonated` true)
          (`self.Spawn Impact Particles` null)
          (`GameplayStatics.ApplyRadialDamageWithFalloff` :`BaseDamage` 10.0 :`MinimumDamage` 10.0 :`Origin` (`self.K2_GetActorLocation` self) :`DamageInnerRadius` 200.0 :`DamageOuterRadius` 300.0 :`DamageTypeClass` "/Game/ShatteredMoon/BluePrints/ExplosionDamage.ExplosionDamage_C" :`DamageCauser` null :`InstigatedByController` null :`DamagePreventionChannel` "ECC_WorldStatic")
          (`ActorComponent.Deactivate` (`self.ParticleSystem`)))))))

(fn `Spawn Impact Particles`
  (params (`Object Hit` :type "Actor Object Reference"))
  (bind _returnvalue (`self.K2_GetActorLocation`))
  (`/Engine/EditorBlueprintResources/StandardMacros.IsValid` `Object Hit`
    (:`Is Valid`
      (if (`self.ActorHasTag` `Object Hit` "Wasp")
        (`GameplayStatics.SpawnEmitterAtLocation` "/Game/ShatteredMoon/Particles/WaspBulletImpact.WaspBulletImpact" _returnvalue (`KismetMathLibrary.Conv_VectorToRotator` (`MovementComponent.Velocity` (`self.ProjectileMovement`))) :!label _label)
        (elif (`self.ActorHasTag` `Object Hit` "enemyWolf")
          (goto _label)
          (elif (`self.ActorHasTag` `Object Hit` "land")
            (`GameplayStatics.PlaySoundAtLocation` "/Game/ShatteredMoon/Audio/SFX/sand_bullet_impact_Gardei.sand_bullet_impact_Gardei" _returnvalue (struct) 0.5 1.0 0.0 null null null)
            (`GameplayStatics.SpawnEmitterAtLocation` "/Game/ShatteredMoon/Particles/sand_bullet_impact.sand_bullet_impact" (+ _returnvalue (0.0 0.0 1.5)))))))))

(fn `UserConstructionScript`
  (bind (_returnvalue_roll _returnvalue_pitch _returnvalue_yaw) (`KismetMathLibrary.BreakRotator` (`self.K2_GetActorRotation`)))
  (bind _target (`self.target`))
  (set `self.randomTarget` (`KismetMathLibrary.MakeVector` (`KismetMathLibrary.RandomFloatInRange` -10000.0 10000.0) (`KismetMathLibrary.RandomFloatInRange` -10000.0 10000.0) (`KismetMathLibrary.RandomFloatInRange` -10000.0 10000.0))) ; This will be the random target projectile will fly towards once target disapears.
  (`/Engine/EditorBlueprintResources/StandardMacros.IsValid` _target
    (:`Is Valid`
      (`self.K2_SetActorRotation` (`KismetMathLibrary.FindLookAtRotation` (`self.K2_GetActorLocation`) (`self.K2_GetActorLocation` _target))))
    (:`Is Not Valid`
      (`self.K2_SetActorRotation` (`KismetMathLibrary.MakeRotator` _returnvalue_roll _returnvalue_pitch (+ _returnvalue_yaw 90.0))))))
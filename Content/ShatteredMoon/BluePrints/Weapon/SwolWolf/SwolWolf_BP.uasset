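; SwolWolf is an easter-egg wolf character that hunts the nearest living Wolf_BP and kills it with massive damage.
; Tick retargets and drives AIMoveTo, with timed hops adding sand puffs and, at long range, random sideways impulses or dodges.
; Other actors can request cooldown-gated dodges through DodgeCheck.
; Damage triggers grunts; death updates GameMode score and enemy counts, then ragdolls and destroys the wolf.
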(event `self.ReceiveBeginPlay`
  ;[1 1 1] On game start... Get Game mode. Needed to get location of VR headset.
  (bind _asshattered_moon_base_mode (cast `/Game/ShatteredMoon/BluePrints/GameMode/ShatteredMoon_BaseMode` (`GameplayStatics.GetGameMode`)))
  (bind _output_get (set `self.gameMode` _asshattered_moon_base_mode))
  (set `CharacterMovementComponent.JumpZVelocity` 200.0 (`self.CharacterMovement`))
  (if (`/Game/ShatteredMoon/BluePrints/GameMode/ShatteredMoon_BaseMode.Wave 3` _output_get)
    (set `self.Health` 40.0)
    (`KismetSystemLibrary.Delay` 1.0) ; its swol... and its a wolf....
    (`GameplayStatics.PlaySound2D` null 1.0 1.0 0.0 null null) ; it's swol, and its a wolf
  ))

(event `self.ReceiveAnyDamage`
  (params (Damage :type "Float (single-precision)") (DamageType :type "DamageType Object Reference") (InstigatedBy :type "Controller Object Reference") (DamageCauser :type "Actor Object Reference"))
  (bind _gamemode (`self.gameMode`))
  (bind _returnvalue (`SceneComponent.K2_GetComponentLocation` (`self.Mesh`)))
  ;[1 1 1] When wolf is hit...
  (if (not (`self.dead`))
    (bind _output_get (set `self.Health` (- (`self.Health`) Damage)))
    (if (<= _output_get 0.0)
      ;;[1 1 1] Kill wolf if health is less than or equal to 0.
      (bind _output_get_2 (set `/Game/ShatteredMoon/BluePrints/GameMode/ShatteredMoon_BaseMode.Enemies Killed` (+ (stale _output_get_2) 1) _gamemode))
      (bind _output_get_3 (set `/Game/ShatteredMoon/BluePrints/GameMode/ShatteredMoon_BaseMode.score` (+ (stale _output_get_3) 150) _gamemode))
      (bind _output_get_4 (set `/Game/ShatteredMoon/BluePrints/GameMode/ShatteredMoon_BaseMode.Enemy Count` (- (stale _output_get_4) 1) _gamemode))
      (`GameplayStatics.SpawnSoundAtLocation` "/Game/ShatteredMoon/Audio/SFX/WolfHit.WolfHit" _returnvalue (struct) 1.0 1.0 0.0 null null)
      (set `self.dead` true)
      (`CharacterMovementComponent.SetMovementMode` (`self.CharacterMovement`) "MOVE_Falling" 0)
      (`PrimitiveComponent.SetSimulatePhysics` (`self.Coyote_V1_Body`) true)
      (`PrimitiveComponent.SetCollisionEnabled` (`self.CapsuleComponent`) "NoCollision")
      (`KismetSystemLibrary.Delay` 3.0)
      (`self.K2_DestroyActor`)
      (else
        ;;[1 1 1] Play Wounded dog noise
        (`GameplayStatics.SpawnSoundAtLocation` "/Game/ShatteredMoon/Audio/SFX/dog_grunt_1_Gardei.dog_grunt_1_Gardei" _returnvalue (struct) 1.0 1.0 0.0 null null)))))

(event `self.ReceiveTick`
  (params (DeltaSeconds :type "Float (single-precision)"))
  (bind _target (`self.target`))
  (bind _speed (`self.speed`))
  (bind _bouncetimer (`self.bounceTimer`))
  (bind _stopbouncetimer (`self.stopBounceTimer`))
  (bind _returnvalue (`KismetMathLibrary.VSizeXY` (- (`self.K2_GetActorLocation`) (`self.playerLocation`))))
  ;[1 1 1] AI Logic
  (if (`self.dead`)
    (`MovementComponent.StopMovementImmediately` (`self.CharacterMovement`))
    (else
      (bind _output_get (set `self.dodgeTimer` (- (stale _output_get) DeltaSeconds)))
      (`self.findClosestTinyWolf`)
      (`/Engine/EditorBlueprintResources/StandardMacros.IsValid` _target
        (:`Is Valid`
          (bind _output_get_2 (set `self.playerLocation` (`self.K2_GetActorLocation` _target)))
          ;;[1 1 1] Run towards player headset.
          (`|AIMoveTo` self _output_get_2 null 1.0
            (:`then`
              (bind _output_get_3 (set `self.bounceTimer` (- _bouncetimer DeltaSeconds)))
              (if (<= _output_get_3 0.0)
                (`self.Jump`)
                (`GameplayStatics.SpawnEmitterAtLocation` "/Game/ShatteredMoon/Particles/sand_bullet_impact.sand_bullet_impact" (`SceneComponent.K2_GetComponentLocation` (`self.DustSocket`))) ; sand particles at feet
                (set `self.bounceTimer` (`self.bounceInterval`))
                (`KismetSystemLibrary.Delay` 0.05) ; allows time for actor to be airborne so 'dodge' impulse doesnt have to fight ground friction
                (if (<= _returnvalue 225.0)
                  (`self.hitWolf` (`self.target`))
                  (elif (<= _returnvalue 2000.0)
                    (`KismetSystemLibrary.PrintString` (`KismetStringLibrary.Conv_DoubleToString` _returnvalue))
                    (elif (`self.canDodge`)
                      (`self.ExecuteDodge`)
                      (else
                        (`self.DodgeWolfCheck`) ; if another wolf is in front of this actor, side step
                        (if (`KismetMathLibrary.RandomBool`)
                          (bind _impulse_vector (`self.ImpulseHelper` _speed -10000.0))
                          (`CharacterMovementComponent.AddImpulse` (`self.CharacterMovement`) _impulse_vector false) ; pulse left
                          (else
                            (bind _impulse_vector_2 (`self.ImpulseHelper` _speed 10000.0))
                            (`CharacterMovementComponent.AddImpulse` (`self.CharacterMovement`) _impulse_vector_2 false) ; pulse right
                          ))))))
                (elif (<= _stopbouncetimer 0.0)
                  (`self.StopJumping`)
                  (set `self.stopBounceTimer` (/ _bouncetimer 2.0))
                  (else
                    (set `self.stopBounceTimer` (- _stopbouncetimer DeltaSeconds))))))))))))

(fn `DodgeCheck`
  (if (<= (stale _output_get) 0.0)
    (bind _output_get (set `self.dodgeTimer` 2.0))
    (set `self.canDodge` true)))

(fn `DodgeWolfCheck`
  (bind _coyote_v1_body (`self.Coyote_V1_Body`))
  (bind _outhit (`KismetSystemLibrary.LineTraceSingle` :`Start` (`SceneComponent.K2_GetComponentLocation` _coyote_v1_body) :`End` (* (`SceneComponent.GetForwardVector` _coyote_v1_body) 2.0) :`TraceChannel` "TraceTypeQuery1" :`DrawTime` 0.0))
  (if (`self.ActorHasTag` (`.HitActor` (`GameplayStatics.BreakHitResult` _outhit)) "enemyWolf")
    (`self.ExecuteDodge`)))

(fn `ExecuteDodge`
  (if (>= (`KismetMathLibrary.VSizeXY` (+ (`self.playerLocation`) (`SceneComponent.K2_GetComponentLocation` (`self.Coyote_V1_Body`)))) 2500.0)
    (set `self.canDodge` false)
    (if (`KismetMathLibrary.RandomBool`)
      (bind _impulse_vector (`self.ImpulseHelper` 5000.0 -50000.0))
      (`CharacterMovementComponent.AddImpulse` (`self.CharacterMovement`) _impulse_vector false) ; bounce left
      (else
        (bind _impulse_vector_2 (`self.ImpulseHelper` 5000.0 50000.0))
        (`CharacterMovementComponent.AddImpulse` (`self.CharacterMovement`) _impulse_vector_2 false) ; bounce right
      ))
    (elif (`KismetMathLibrary.RandomBool`)
      (bind _impulse_vector_3 (`self.ImpulseHelper` 0.0 -10000.0))
      (`CharacterMovementComponent.AddImpulse` (`self.CharacterMovement`) _impulse_vector_3 false) ; bounce left
      (else
        (bind _impulse_vector_4 (`self.ImpulseHelper` 0.0 10000.0))
        (`CharacterMovementComponent.AddImpulse` (`self.CharacterMovement`) _impulse_vector_4 false) ; bounce right
      ))))

(fn `findClosestTinyWolf`
  (bind _outactors (`GameplayStatics.GetAllActorsOfClass` "/Game/ShatteredMoon/BluePrints/Enemy/Wolf_BP.Wolf_BP_C"))
  (if (== (`KismetArrayLibrary.Array_Length` _outactors) 0)
    (if (`self.EnemyNotDetected`)
      (set `self.EnemyNotDetected` true)
      (else
        (set `self.EnemyNotDetected` false :!label _label)))
    (else
      (set `self.Shortest Distance` 100000000376832.0)
      (for _array_element _outactors
        (bind _returnvalue (`self.GetDistanceTo` _array_element))
        (if (< _returnvalue (`self.Shortest Distance`))
          (if (not (`/Game/ShatteredMoon/BluePrints/Enemy/Wolf_BP.dead` _array_element))
            (set `self.target` _array_element)
            (set `self.Shortest Distance` _returnvalue))))
      (goto _label))))

(fn `hitWolf`
  (params (Target :type "Actor Object Reference"))
  (bind _returnvalue (`self.K2_GetActorLocation` Target))
  (bind _aswolf_bp (cast `/Game/ShatteredMoon/BluePrints/Enemy/Wolf_BP` Target))
  (if (not (`/Game/ShatteredMoon/BluePrints/Enemy/Wolf_BP.dead` _aswolf_bp))
    (`GameplayStatics.ApplyDamage` Target 9001.0 null null "/Script/Engine.DamageType") ; its over 9000!
    (if (< (`KismetMathLibrary.VSizeXY` (- (`self.K2_GetActorLocation` Target) (`PlayerCameraManager.GetCameraLocation` (`GameplayStatics.GetPlayerCameraManager` 0)))) 2000.0)
      (`GameplayStatics.SpawnEmitterAtLocation` "/Game/ShatteredMoon/Particles/TurretDeploy.TurretDeploy" _returnvalue (struct) (0.25 0.25 0.25))
      (else
        (`GameplayStatics.SpawnEmitterAtLocation` "/Game/ShatteredMoon/Particles/TurretDeploy.TurretDeploy" _returnvalue (struct) (1.5 1.5 1.5))))))

(fn `ImpulseHelper`
  (params (`Forward Impulse` :type "Float (double-precision)") (`Side Impulse` :type "Float (double-precision)"))
  (returns (`Impulse Vector` :type "Vector Structure"))
  (bind _returnvalue (`self.K2_GetActorRotation`))
  (return (+ (`self.GetVelocity`) (+ (* (`KismetMathLibrary.GetRightVector` _returnvalue) `Side Impulse`) (* (`KismetMathLibrary.GetForwardVector` _returnvalue) `Forward Impulse`)))))

(fn `UserConstructionScript`
  (bind _outactors (`GameplayStatics.GetAllActorsOfClass` "/Game/VirtualRealityBP/Blueprints/MotionControllerPawn.MotionControllerPawn_C"))
  (set `self.player` (`|GetArrayItem` _outactors)))